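; BP_Puzzle is an actor that builds the board for a sliding picture puzzle at BeginPlay; it contains no tile-moving logic.
; SpawnPuzzle lays out a GridSize square grid, adding a box component per cell and a mesh tile in all but the last, leaving one empty space.
; Each tile's dynamic material receives the shared texture plus a UV offset and scale, so it shows its slice of the image.
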(event `self.ReceiveBeginPlay`
  (`self.SpawnPuzzle`))

(fn `SpawnPuzzle`
  (bind _meshsize (`self.MeshSize`))
  (bind _meshsize_2 (`self.MeshSize`))
  (bind _returnvalue (- (`self.GridSize`) 1))
  (bind _returnvalue_2 (/ (`self.MeshSize`) 4.0))
  (bind _returnvalue_3 (- (`self.GridSize`) 1))
  (bind _returnvalue_4 (/ 1.0 (`KismetMathLibrary.Conv_IntToDouble` (`self.GridSize`))))
  (for _index (range (+ _returnvalue 1))
    (set `self.Y Index` _index)
    (for _index_2 (range (+ _returnvalue 1))
      (set `self.X Index` _index_2)
      (bind _returnvalue_5 (`AddComponent|NODE_AddBoxComponent-0` :`RelativeTransform` (`KismetMathLibrary.MakeTransform` (`KismetMathLibrary.MakeVector` (* (`self.X Index`) _meshsize) (* (`self.Y Index`) _meshsize)))))
      (`BoxComponent.SetBoxExtent` _returnvalue_5 (`KismetMathLibrary.MakeVector` _returnvalue_2 _returnvalue_2 _returnvalue_2) true)
      (`KismetArrayLibrary.Array_Add` (`self.SpacesList`) _returnvalue_5)
      (if (not (and (== (`self.X Index`) _returnvalue_3) (== _returnvalue_3 (`self.Y Index`))))
        (bind _returnvalue_6 (`AddComponent|NODE_AddStaticMeshComponent-0` :`RelativeTransform` (`KismetMathLibrary.MakeTransform` (`KismetMathLibrary.MakeVector` (* (`self.X Index`) _meshsize_2) (* (`self.Y Index`) _meshsize_2)))))
        (`KismetArrayLibrary.Array_Add` (`self.MeshesList`) _returnvalue_6)
        (bind _returnvalue_7 (`PrimitiveComponent.CreateDynamicMaterialInstance` _returnvalue_6 0 "/Game/SlidePuzzle/M_PuzzleMaterial.M_PuzzleMaterial" "None"))
        (`MaterialInstanceDynamic.SetTextureParameterValue` _returnvalue_7 "PuzzleTexture" (`self.Texture`))
        (`MeshComponent.SetVectorParameterValueOnMaterials` _returnvalue_6 "TextureOffset2D" (`KismetMathLibrary.MakeVector` (* (`self.X Index`) _returnvalue_4) (* (`self.Y Index`) _returnvalue_4) _returnvalue_4))))))

(fn `UserConstructionScript`)