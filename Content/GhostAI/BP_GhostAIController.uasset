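; BP_GhostAIController is the AI controller for a ghost that keeps track of the player.
; On BeginPlay it runs the assigned behavior tree.
; Every tick it writes the player pawn and its location to the Player and PlayerLocation blackboard keys and sets focus on that pawn.
; An AIMoveTo node is present but never runs.
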(event `self.ReceiveBeginPlay`
  (`self.RunBehaviorTree` (`self.BTAsset`)))

(event `self.ReceiveTick`
  (params (DeltaSeconds :type "Float (single-precision)"))
  (bind _returnvalue (`GameplayStatics.GetPlayerPawn` 0))
  (`BlackboardComponent.SetValueAsObject` (`AIBlueprintHelperLibrary.GetBlackboard` null) "Player" _returnvalue)
  (`BlackboardComponent.SetValueAsVector` (`AIBlueprintHelperLibrary.GetBlackboard` null) "PlayerLocation" (`self.K2_GetActorLocation` (`GameplayStatics.GetPlayerPawn` 0)))
  (`self.K2_SetFocus` _returnvalue))

(fn `UserConstructionScript`)