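; BP_Ghost is an AI-controlled ghost that can be warded, making it avoidant.
; The Warded event sets the Avoidant flag and copies it to the "Avoidant?" Blackboard key through BP_GhostAIController.
; A retriggerable delay of DefaultWardedTime then clears the flag, so repeated wards restart the timer.
; The reset changes only the local variable and does not write back to the Blackboard.
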(event `Warded`
  (set `self.Avoidant` true)
  (bind _asbp_ghost_aicontroller (cast `/Game/GhostAI/BP_GhostAIController` (`AIBlueprintHelperLibrary.GetAIController` self)))
  (`BlackboardComponent.SetValueAsBool` (`AIController.Blackboard` _asbp_ghost_aicontroller) "Avoidant?" (`self.Avoidant`))
  (`KismetSystemLibrary.RetriggerableDelay` (`self.Default Warded Time`))
  (set `self.Avoidant` false))

(fn `UserConstructionScript`)